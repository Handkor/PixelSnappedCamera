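; Pixel-perfect orthographic camera that becomes the player view and follows a target actor at its initial offset.
; Each tick it snaps its scene capture, and components supplied by PixelSnappableInterface actors, to a camera-aligned grid of ViewSize/Resolution and to rotation steps.
; Only components move, so actor transforms stay unsnapped.
; It then captures the scene manually and draws M_Transform into RT_Final.
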(event `self.ReceiveBeginPlay`
  (`PlayerController.SetViewTargetWithBlend` (`GameplayStatics.GetPlayerController` 0) self 0.0 "VTBlend_Linear" 0.0 false))

(event `self.ReceiveTick`
  (params (DeltaSeconds :type "Float (single-precision)"))
  (bind _actortofollow (`self.ActorToFollow`))
  (`|ExecutionSequence`
    (:`then_0`
      (`/Engine/EditorBlueprintResources/StandardMacros.IsValid` _actortofollow
        (:`Is Valid`
          (`self.K2_SetActorLocation` (+ (`self.K2_GetActorLocation` _actortofollow) (`self.Offset`)) false true))))
    (:`then_1`
      (`self.SnapComponentToView` self (`self.SceneCaptureComponent2D`)))
    (:`then_2`
      (bind _outactors (`GameplayStatics.GetAllActorsWithInterface` "/Game/PixelSnappedCamera/PixelSnappableInterface.PixelSnappableInterface_C"))
      (for _array_element _outactors
        (bind _snapped_component (message `/Game/PixelSnappedCamera/PixelSnappableInterface.GetSnappedComponent` _array_element))
        (`self.SnapComponentToView` _array_element _snapped_component)))
    (:`then_3`
      (`SceneCaptureComponent2D.CaptureScene` (`self.SceneCaptureComponent2D`))
      (`KismetRenderingLibrary.DrawMaterialToRenderTarget` "/Game/PixelSnappedCamera/RT_Final.RT_Final" "/Game/PixelSnappedCamera/M_Transform.M_Transform"))))

(fn `SnapComponentToView`
  (params (Actor :type "Actor Object Reference") (Component :type "SceneComponent Object Reference"))
  (bind _rotationsnaps (`self.RotationSnaps`))
  (bind _returnvalue (/ (`self.ViewSize`) (`self.Resolution`)))
  (bind _returnvalue_2 (`KismetMathLibrary.MakeTransform` (0.0 0.0 0.0) (.rotation (`self.GetTransform`)) (.scale (`self.GetTransform`))))
  (`|ExecutionSequence`
    (:`then_0`
      (`SceneComponent.K2_SetWorldLocation` Component (`KismetMathLibrary.TransformLocation` _returnvalue_2 (`KismetMathLibrary.MakeVector` (`KismetMathLibrary.GridSnap_Float` (.x (`KismetMathLibrary.InverseTransformLocation` _returnvalue_2 (`self.K2_GetActorLocation` Actor))) _returnvalue) (`KismetMathLibrary.GridSnap_Float` (.y (`KismetMathLibrary.InverseTransformLocation` _returnvalue_2 (`self.K2_GetActorLocation` Actor))) _returnvalue) (`KismetMathLibrary.GridSnap_Float` (.z (`KismetMathLibrary.InverseTransformLocation` _returnvalue_2 (`self.K2_GetActorLocation` Actor))) _returnvalue))) false true))
    (:`then_1`
      (`SceneComponent.K2_SetWorldRotation` Component (`KismetMathLibrary.MakeRotator` (`KismetMathLibrary.GridSnap_Float` (.roll (`self.K2_GetActorRotation` Actor)) _rotationsnaps) (`KismetMathLibrary.GridSnap_Float` (.pitch (`self.K2_GetActorRotation` Actor)) _rotationsnaps) (`KismetMathLibrary.GridSnap_Float` (.yaw (`self.K2_GetActorRotation` Actor)) _rotationsnaps)) false true))))

(fn `SnapMovementToView`
  (params (`New Location` :type "Vector Structure"))
  (returns (Out :type "Vector Structure"))
  (bind _returnvalue (`KismetMathLibrary.MakeTransform` (0.0 0.0 0.0) (.rotation (`self.GetTransform`)) (.scale (`self.GetTransform`))))
  (bind _x (.x (`KismetMathLibrary.InverseTransformLocation` _returnvalue (- `New Location` (.location (`self.GetTransform`))))))
  (bind _y (.y (`KismetMathLibrary.InverseTransformLocation` _returnvalue (- `New Location` (.location (`self.GetTransform`))))))
  (bind _z (.z (`KismetMathLibrary.InverseTransformLocation` _returnvalue (- `New Location` (.location (`self.GetTransform`))))))
  (bind _returnvalue_2 (`KismetMathLibrary.FMax` (`KismetMathLibrary.Abs` _x) (`KismetMathLibrary.Abs` _y) (`KismetMathLibrary.Abs` _z)))
  (return (+ (`self.K2_GetActorLocation`) (`KismetMathLibrary.TransformLocation` _returnvalue (`KismetMathLibrary.MakeVector` (* _returnvalue_2 (select `bool` (!= _x 0.0) :`true` (`KismetMathLibrary.SignOfFloat` _x))) (* _returnvalue_2 (select `bool` (!= _y 0.0) :`true` (`KismetMathLibrary.SignOfFloat` _y))) (* _returnvalue_2 (select `bool` (!= _z 0.0) :`true` (`KismetMathLibrary.SignOfFloat` _z))))))))

(fn `UserConstructionScript`
  (set `SceneCaptureComponent2D.OrthoWidth` (`self.ViewSize`) (`self.SceneCaptureComponent2D`))
  (bind _returnvalue (`PrimitiveComponent.CreateDynamicMaterialInstance` (`self.Plane`) 0 null))
  (`MaterialInstanceDynamic.SetScalarParameterValue` _returnvalue "Resolution" (`self.Resolution`))
  (`/Engine/EditorBlueprintResources/StandardMacros.IsValid` (`self.ActorToFollow`)
    (:`Is Valid`
      (set `self.Offset` (- (`self.K2_GetActorLocation`) (`self.K2_GetActorLocation` (`self.ActorToFollow`)))))))